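; In-game player controller for SimpleRacer that handles the pause menu and switching between character and vehicle input.
; The toggle-menu input lazily creates W_MainMenu on first use, then flips its visibility along with game pause, mouse cursor and input mode.
; Two functions swap the character and vehicle Enhanced Input mapping contexts.
; DoSomethingForAnimation is a placeholder that only prints a debug string.
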(event Input|EnhancedActionEvents|EnhancedInputActionIA_ToggleMenu
  (params (ActionValue :type Boolean) (ElapsedSeconds :type Float%20%28double-precision%29) (TriggeredSeconds :type Float%20%28double-precision%29) (InputAction :type Input%20Action%20Object%20Reference :default "/Game/SimpleRacer/Core/Input/Actions/IA_ToggleMenu.IA_ToggleMenu"))
  (bind _self self)
  (bind _self_2 self)
  (:Triggered
    (bind _menuwidget (Variables|Default|GetMenuWidget)
      (:then
        (switch Utilities|FlowControl|Switch|SwitchonESlateVisibility (Widget|GetVisibility _menuwidget)
          (:Visible
            (Widget|SetVisibility _menuwidget "Collapsed" :!label _label)
            (Input|SetInputModeGameOnly _self false)
            (Variables|Default|SetbShowMouseCursor _self false)
            (Game|SetGamePaused false))
          (:Collapsed
            (Widget|SetVisibility _menuwidget "Visible" :!label _label_2)
            (Input|SetInputModeGameandUI _self_2 0 "DoNotLock" true false :!label _label_3)
            (Variables|Default|SetbShowMouseCursor _self_2 true)
            (Game|SetGamePaused true))
          (:Hidden
            (goto _label_2))
          (:HitTestInvisible
            (goto _label))
          (:SelfHitTestInvisible
            (goto _label))))
      (:else
        (bind _returnvalue (UserInterface|CreateWidget "/Game/SimpleRacer/UI/W_MainMenu.W_MainMenu_C"))
        (bind _output_get (Variables|Default|SetMenuWidget _returnvalue))
        (UserInterface|Viewport|AddtoViewport _output_get 0)
        (goto _label_3)))))

(event EventBeginPlay
  (Input|SetInputModeGameOnly self false))

(fn ConstructionScript)

(fn DoSomethingforAnimation
  (Development|PrintString "Hello"))

(fn SwitchtoVehicleControls
  (bind _returnvalue (PlayerController|LocalPlayerSubsystems|GetEnhancedInputLocalPlayerSubsystem))
  (Utilities|IsValid _returnvalue
    (:Is%20Valid
      (Input|RemoveMappingContext _returnvalue "/Game/SimpleRacer/Core/Input/IMC_Character.IMC_Character" "(bIgnoreAllPressedKeysUntilRelease=True,bForceImmediately=False)")
      (Input|AddMappingContext _returnvalue "/Game/SimpleRacer/Core/Input/IMC_Vehicle.IMC_Vehicle" 0 "(bIgnoreAllPressedKeysUntilRelease=True,bForceImmediately=False)"))))

(fn SwitchtoCharacterControls
  (bind _returnvalue (PlayerController|LocalPlayerSubsystems|GetEnhancedInputLocalPlayerSubsystem))
  (Utilities|IsValid _returnvalue
    (:Is%20Valid
      (Input|RemoveMappingContext _returnvalue "/Game/SimpleRacer/Core/Input/IMC_Vehicle.IMC_Vehicle" "(bIgnoreAllPressedKeysUntilRelease=True,bForceImmediately=False)")
      (Input|AddMappingContext _returnvalue "/Game/SimpleRacer/Core/Input/IMC_Character.IMC_Character" 0 "(bIgnoreAllPressedKeysUntilRelease=True,bForceImmediately=False)"))))
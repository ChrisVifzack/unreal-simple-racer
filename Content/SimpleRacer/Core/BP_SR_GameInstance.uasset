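; Game instance for SimpleRacer that keeps the last and best race times and persists the best time between sessions.
; On Init it loads the best time from the save slot, if a save exists.
; UpdateScore records each new race time and saves it when it beats the best or no best is set.
; Saving updates the existing BP_SaveGame in the slot or creates a new one.
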(event EventInit
  (CallFunction|TryLoadGame))

(fn UpdateScore
  (params (NewRaceTime :type Float%20%28double-precision%29))
  (Variables|Default|SetLastRaceTime NewRaceTime)
  (if (or (< NewRaceTime (Variables|Default|GetBestRaceTime)) (<= (Variables|Default|GetBestRaceTime) 0.0))
    (Variables|Default|SetBestRaceTime NewRaceTime)
    (CallFunction|SaveGame)))

(fn SaveGame
  (bind _returnvalue (SaveGame|DoesSaveGameExist "Slot"))
  (if _returnvalue
    (bind _returnvalue_2 (SaveGame|LoadGamefromSlot "Slot"))
    (bind _asbp_save_game (Utilities|Casting|CastToBP_SaveGame _returnvalue_2))
    (Variables|/Game/SimpleRacer/Core/SaveGame/BP_SaveGame.BP_SaveGame_C|SetBestRaceTime _asbp_save_game (Variables|Default|GetBestRaceTime))
    (SaveGame|SaveGametoSlot _asbp_save_game "Slot")
    (else
      (bind _returnvalue_3 (SaveGame|CreateSaveGameObject "/Game/SimpleRacer/Core/SaveGame/BP_SaveGame.BP_SaveGame_C"))
      (Variables|/Game/SimpleRacer/Core/SaveGame/BP_SaveGame.BP_SaveGame_C|SetBestRaceTime _returnvalue_3 (Variables|Default|GetBestRaceTime))
      (SaveGame|SaveGametoSlot _returnvalue_3 "Slot"))))

(fn TryLoadGame
  (bind _returnvalue (SaveGame|DoesSaveGameExist "Slot"))
  (if _returnvalue
    (bind _returnvalue_2 (SaveGame|LoadGamefromSlot "Slot"))
    (bind _asbp_save_game (Utilities|Casting|CastToBP_SaveGame _returnvalue_2))
    (Variables|Default|SetBestRaceTime (Variables|/Game/SimpleRacer/Core/SaveGame/BP_SaveGame.BP_SaveGame_C|GetBestRaceTime _asbp_save_game))))
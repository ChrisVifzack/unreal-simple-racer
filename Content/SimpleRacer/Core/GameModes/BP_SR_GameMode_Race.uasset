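; Race game mode for SimpleRacer that times a run through numbered checkpoints and shows the time in a race UI widget.
; BeginPlay counts placed checkpoints, creates the UI and loads saved data through the game instance.
; The first checkpoint hit starts the timer, and only the expected checkpoint advances progress and broadcasts the new active one.
; After the last, it submits the time to the game instance and loads MainMenu as a level instance.
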(event Custom|CheckpointPassed
  (params (CheckpointNum :type Integer) (Checkpoint :type BP%20Checkpoint%20Object%20Reference))
  (bind _nextcheckpointnum (Variables|Default|GetNextCheckpointNum))
  (Development|PrintString "Checkpoint Passed")
  (Utilities|FlowControl|Sequence
    (:then_0
      (if (== (Variables|Default|GetNextCheckpointNum) 0)
        (Utilities|FlowControl|DoOnce false
          (:Completed
            (CallFunction|StartRace)
            (Development|PrintString "Start Race" true true "(R=0.042621,G=1.000000,B=0.000000,A=1.000000)")))))
    (:then_1
      (if (== (Variables|Default|GetNextCheckpointNum) CheckpointNum)
        (Math|Integer|IncrementInt _nextcheckpointnum
          (:%20%20
            (Default|CallOnActiveCheckpointChanged _nextcheckpointnum)
            (if (not (< _nextcheckpointnum (Variables|Default|GetMaxCheckpointNum)))
              (CallFunction|EndRace)
              (Development|PrintString "Finish Race" true true "(R=1.000000,G=0.051495,B=0.000000,A=1.000000)"))))))))

(event EventBeginPlay
  (|CallParentFunction)
  (bind _outactors (Actor|GetAllActorsOfClass "/Game/SimpleRacer/Gameplay/BP_Checkpoint.BP_Checkpoint_C"))
  (Variables|Default|SetCheckpoints _outactors)
  (Variables|Default|SetMaxCheckpointNum (Utilities|Array|Length _outactors))
  (bind _returnvalue (UserInterface|CreateWidget "/Game/SimpleRacer/UI/W_RaceUI.W_RaceUI_C" (Game|GetPlayerController 0)))
  (bind _output_get (Variables|Default|SetRace_UI _returnvalue))
  (UserInterface|Viewport|AddtoViewport _output_get 0)
  (bind _asbp_sr_game_instance (Utilities|Casting|CastToBP_SR_GameInstance (Game|GetGameInstance)))
  (Default|TryLoadGame _asbp_sr_game_instance))

(event EventTick
  (params (DeltaSeconds :type Float%20%28single-precision%29))
  (bind _race_ui (Variables|Default|GetRace_UI))
  (Utilities|IsValid _race_ui
    (:Is%20Valid
      (Default|UpdateTime _race_ui (Math|Timespan|FromSeconds (CallFunction|GetRaceTime))))))

(fn ConstructionScript
  (|CallParentFunction))

(fn EndRace
  (Variables|Default|SetFinishTime (Utilities|Time|GetTimeSeconds))
  (Variables|Default|SetbIsTrackingTime false)
  (bind _asbp_sr_game_instance (Utilities|Casting|CastToBP_SR_GameInstance (Game|GetGameInstance)))
  (Default|UpdateScore _asbp_sr_game_instance (CallFunction|GetRaceTime))
  (Class|LevelStreamingDynamic|LoadLevelInstancebySoftObjectPtr "/Game/SimpleRacer/Maps/Menu/MainMenu.MainMenu" "0, 0, 0" "0, 0, 0" "" 0 false))

(fn StartRace
  (Variables|Default|SetInitialTime (Utilities|Time|GetTimeSeconds))
  (Variables|Default|SetbIsTrackingTime true))

(fn GetRaceTime
  (if (Variables|Default|GetbIsTrackingTime)
    (return (- (Utilities|Time|GetTimeSeconds) (Variables|Default|GetInitialTime)))
    (else
      (return (- (Variables|Default|GetFinishTime) (Variables|Default|GetInitialTime))))))